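; BP_GoldMine is a clickable gold mine prop that plays a one-shot skeletal death animation and timeline, then destroys itself.
; Hovering traces under the mouse and spawns an emitter at the hit point, throttled by a delayed DoOnce reset.
; Its construction script optionally box-traces to snap and align the actor to the Landscape, and can randomly rotate the mesh, each toggled by a boolean.
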(event EventBeginPlay)

(event Collision|EventActorBeginOverlap
  (params (OtherActor :type Actor%20Object%20Reference)))

(event EventTick
  (params (DeltaSeconds :type Float%20%28single-precision%29)))

(event MouseInput|EventActorBeginCursorOver
  (bind _returnvalue (Game|GetPlayerController 0))
  (bind (_worldlocation _worlddirection) (Game|Player|ConvertMouseLocationToWorldSpace _returnvalue))
  ;[1 1 1] Get mouse location on Actor
  (bind _outhit (Collision|LineTraceByChannel (+ _worldlocation _worlddirection) (+ _worldlocation (* _worlddirection 4000)) "TraceTypeQuery1" true 0 "None" false))
  ;[1 1 1] Spawn Particles on mouse location
  (if (stale MouseInput|EventActorOnClicked _output_get)
    _
    (else
      _))
  (Utilities|FlowControl|DoOnce false :!label _label
    (:Completed
      (Utilities|FlowControl|Delay 1.0)
      (Effects|SpawnEmitteratLocation 0 (.ImpactPoint (Collision|BreakHitResult _outhit)) (Math|Conversions|RotationFromXVector (.ImpactNormal (Collision|BreakHitResult _outhit))))
      (goto _label Reset))))

(event MouseInput|EventActorOnClicked
  (params (ButtonPressed :type Key%20Structure))
  ;[1 1 1] Play Dead Animation on Clicked
  (Utilities|FlowControl|DoOnce false
    (:Completed
      (bind _output_get (Variables|Default|SetbAutoDestroyWhenFinished true))
      (Components|Animation|PlayAnimation (Variables|SkeletalMeshActor|GetSkeletalMeshComponent) "/Game/CartoonRtsFoliage/Meshes/GoldMines/SK_GoldMIne_01_Anim.SK_GoldMIne_01_Anim" false)
      (Timeline|GoldMine_Timeline Play
        (:Finished
          (Actor|DestroyActor))))))

(fn ConstructionScript
  ;[1 1 1] Set Booleans to easily trigger the construction script or disable the update pos with the landscape
  (if (Variables|Default|GetUpdatePos)
    (CallFunction|UpdatePosition))
  (if (Variables|Default|GetActivateConstructionScript)
    (CallFunction|ParentTransforms)))

(fn ParentTransforms
  (bind _returnvalue (Math|Random|RandomFloatinRange 0.0 1e+01))
  ;[1 1 1] Randomly rotate the skeletal mesh
  (Transformation|SetWorldRotation (Variables|SkeletalMeshActor|GetSkeletalMeshComponent) (Math|Rotator|MakeRotator _returnvalue _returnvalue (Math|Random|RandomFloatinRange 0.0 3.6e+02)) false false))

(fn UpdatePosition
  (bind _returnvalue (Transformation|GetActorLocation))
  ;[1 1 1] Check with a boxTrace The actor location with the landscape
  (bind _outhit (Collision|BoxTraceByChannel (+ _returnvalue "0, 0,5000.000000") (- _returnvalue (Math|Vector|MakeVector 0.0 0.0 5e+03)) "25.000000,25.000000,10.000000" "0, 0, 0" "TraceTypeQuery3" false 0 "None"))
  ;[1 1 1] Align the mesh with the landscape
  (if (== (Utilities|GetClass (.HitActor (Collision|BreakHitResult _outhit))) "/Script/Landscape.Landscape")
    (Transformation|SetActorLocation (+ (.Location (Collision|BreakHitResult _outhit)) (Variables|Default|GetTreeOfset)) false false)
    (Transformation|SetActorRotation (Math|Rotator|MakeRotfromZ (.Normal (Collision|BreakHitResult _outhit))))))
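; AI controller for miner units (BP_Miner) that starts their BT_Miner behavior tree and supplies its mining locations.
; Its Ready event writes the location of the first BP_Ore found in the level to the TargetOre blackboard key, and the pawn's owner building location to Owner.
; The behavior tree is run both before and after these blackboard writes, and Tick is empty.
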(event EventTick
  (params (DeltaSeconds :type Float%20%28single-precision%29)))

(event EventReady
  (bind _returnvalue (AI|GetBlackboard 0))
  (AI|RunBehaviorTree "/Game/WW4/Blueprint/AI/BT_Miner.BT_Miner")
  (bind _returnvalue_2 (Actor|GetActorOfClass "/Game/WW4/Blueprint/Ore/BP_Ore.BP_Ore_C"))
  (AI|Components|Blackboard|SetValueasVector _returnvalue (Utilities|Name|MakeLiteralName "TargetOre") (Transformation|GetActorLocation _returnvalue_2))
  (AI|Components|Blackboard|SetValueasVector _returnvalue (Utilities|Name|MakeLiteralName "Owner") (Transformation|GetActorLocation (Class|UnitBase|GetOwnerBuilding (.AsBP%20Miner (Utilities|Casting|CastToBP_Miner (Pawn|GetControlledPawn))))))
  (AI|RunBehaviorTree "/Game/WW4/Blueprint/AI/BT_Miner.BT_Miner"))

(fn ConstructionScript)
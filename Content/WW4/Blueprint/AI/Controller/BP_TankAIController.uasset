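; AI controller for tank units that picks an initial destination and handles move pausing around perceived units.
; Shortly after BeginPlay it runs a spawn-point EQS query, floor-traces the result and sends the move through the player controller's base component.
; Perception updates pause movement when a unit is sensed and resume it when that tracked unit is lost.
; Perception is deactivated at BeginPlay and not reactivated here.
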(event OnTargetPerceptionUpdated(AIPerception)
  (params (Actor :type Actor%20Object%20Reference) (Stimulus :type AI%20Stimulus%20Structure))
  (bind _bsuccessfullysensed (Utilities|Struct|BreakAIStimulus Stimulus))
  (bind _asunit_base (Utilities|Casting|CastToUnitBase Actor))
  (Utilities|IsValid (Variables|Default|Gettemp)
    (:Is%20Valid
      (if (== (Variables|Default|Gettemp) _asunit_base)
        (if (not _bsuccessfullysensed)
          (bind _returnvalue (Class|UnitAIControllerBase|ReusmeCurrentMove))
          (if _returnvalue
            (Variables|Default|Settemp 0)))
        (else
          (if _bsuccessfullysensed :!label _label
            (bind _returnvalue_2 (Class|UnitAIControllerBase|PauseCurrentMove))
            (if _returnvalue_2
              (Variables|Default|Settemp _asunit_base))))))
    (:Is%20Not%20Valid
      (goto _label))))

(event Custom|OnQueryFinishedEvent_Event
  (params (QueryInstance :type Env%20Query%20Instance%20Blueprint%20Wrapper%20Object%20Reference) (QueryStatus :type EEnvQueryStatus%20Enum :default "Processing"))
  (bind (_resultlocations _returnvalue) (AI|EQS|GetQueryResultsasLocations QueryInstance))
  (if _returnvalue
    (bind _outhitresult (Class|WW4CommonFunctionLibrary|TraceFloorUnderWorldLocation (Utilities|Array|Get(acopy) _resultlocations)))
    (Class|PlayerBaseComponent|ServerMoveUnit (Variables|/Script/WW4.WW4PlayerController|GetPlayerBaseComponent (Class|WW4CommonFunctionLibrary|GetWW4PlayerController)) (.AsUnit%20Base (Utilities|Casting|CastToUnitBase (Pawn|GetControlledPawn))) (.Location (Collision|BreakHitResult _outhitresult)))))

(event EventBeginPlay
  (Components|Activation|Deactivate (Variables|Default|GetAIPerception))
  (Utilities|FlowControl|Delay 0.1)
  (bind _returnvalue (AI|EQS|RunEQSQuery "/Game/WW4/Blueprint/AI/EQS/EQS_UnitFindSpawnPoint.EQS_UnitFindSpawnPoint" self "RandomBest5Pct"))
  (EventDispatchers|AssignOnQueryFinishedEvent _returnvalue (delegate Custom|OnQueryFinishedEvent_Event)))

(event EventTick
  (params (DeltaSeconds :type Float%20%28single-precision%29)))

(fn ConstructionScript)
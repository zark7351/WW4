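; Tank AI controller that halts the tank's current move when perception senses a UnitBase and resumes it when that unit is lost.
; Perception updates drive pause and resume calls, with Temp remembering the unit behind the pause.
; Sensing a different unit replaces Temp if the pause succeeds, and only losing the stored unit can resume movement and clear it.
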(event OnTargetPerceptionUpdated(AIPerception)
  (params (Actor :type Actor%20Object%20Reference) (Stimulus :type AI%20Stimulus%20Structure))
  (bind _bsuccessfullysensed (Utilities|Struct|BreakAIStimulus Stimulus))
  (bind _asunit_base (Utilities|Casting|CastToUnitBase Actor))
  (Utilities|IsValid (Variables|Default|Gettemp)
    (:Is%20Valid
      (if (== (Variables|Default|Gettemp) _asunit_base)
        (if (not _bsuccessfullysensed)
          (bind _returnvalue (Class|UnitAIControllerBase|ReusmeCurrentMove))
          (if _returnvalue
            (Variables|Default|Settemp 0)))
        (else
          (if _bsuccessfullysensed :!label _label
            (bind _returnvalue_2 (Class|UnitAIControllerBase|PauseCurrentMove))
            (if _returnvalue_2
              (Variables|Default|Settemp _asunit_base))))))
    (:Is%20Not%20Valid
      (goto _label))))

(event EventBeginPlay)

(event EventTick
  (params (DeltaSeconds :type Float%20%28single-precision%29)))

(fn ConstructionScript)
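; BP_BuildingConstructor is a mouse-driven placement cursor for constructing buildings on a grid.
; Each tick it traces under the mouse, snaps the target to 100-unit XY steps and interpolates toward it.
; AddChildren attaches a 5x5 block of BP_BuildingGridCell actors, and CanConstruct checks for enabled, blocked cells.
; BPConstruct, when unblocked, spawns the selected building's class from DT_BuildingInfo, then destroys the constructor.
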(event Custom|BPConstruct
  (bind _can (CallFunction|CanConstruct))
  (if _can
    (bind _returnvalue (Utilities|GetDataTableRow "/Game/WW4/Datatable/DT_BuildingInfo.DT_BuildingInfo" (Utilities|String|StringToName (Variables|Default|GetCurBuilding)))
      (:then
        (Game|SpawnActorfromClass (.ItemClass (Utilities|Struct|BreakBuildingProductionInfo _returnvalue)) (Math|Transform|MakeTransform (+ (Variables|Default|GetLastPost) "0.000000,0.000000,0.500000")) "Undefined" "MultiplyWithRoot" 0 0)
        (for _array_element 0
          (Actor|DestroyActor _array_element))
        (Variables|/Script/Engine.PlayerController|SetbShowMouseCursor (Game|GetPlayerController 0) true)
        (Actor|DestroyActor)))))

(event Collision|EventActorBeginOverlap
  (params (OtherActor :type Actor%20Object%20Reference)))

(event EventTick
  (params (DeltaSeconds :type Float%20%28single-precision%29))
  (Utilities|FlowControl|Sequence
    (:then_0
      (CallFunction|UpdatePos))
    (:then_1
      (Transformation|SetActorLocation (Math|Interpolation|VInterpTo (Transformation|GetActorLocation) (Variables|Default|GetLastPost) DeltaSeconds 2e+01) false false))))

(fn ConstructionScript)

(fn Trace
  (bind _returnvalue (Class|WidgetLayoutLibrary|GetMousePositiononViewport))
  (bind (_outhit _returnvalue_2) (Collision|LineTraceForObjects (.WorldPosition (Class|GameplayStatics|DeprojectScreentoWorld (Game|GetPlayerController 0) (* _returnvalue (Class|WidgetLayoutLibrary|GetViewportScale)))) (+ (.WorldPosition (Class|GameplayStatics|DeprojectScreentoWorld (Game|GetPlayerController 0) (* _returnvalue (Class|WidgetLayoutLibrary|GetViewportScale)))) (* (.WorldDirection (Class|GameplayStatics|DeprojectScreentoWorld (Game|GetPlayerController 0) (* _returnvalue (Class|WidgetLayoutLibrary|GetViewportScale)))) 1e+05)) (Utilities|Array|MakeArray "ObjectTypeQuery7") false 0 "None"))
  (return _outhit _returnvalue_2))

(fn UpdatePos
  (bind (_outhit _returnvalue) (CallFunction|Trace))
  (if _returnvalue
    (if (or (>= (Math|Float|Absolute(Float) (- (.X (Math|Vector|BreakVector (.Location (Collision|BreakHitResult _outhit)))) (.x (Variables|Default|GetLastPost)))) 1e+02) (>= (Math|Float|Absolute(Float) (- (.y (Variables|Default|GetLastPost)) (.Y (Math|Vector|BreakVector (.Location (Collision|BreakHitResult _outhit)))))) 1e+02))
      (Variables|Default|SetLastPost (Math|Vector|MakeVector (Math|Conversions|ToFloat(Integer) (* (Class|KismetMathLibrary|Round64 (/ (.X (Math|Vector|BreakVector (.Location (Collision|BreakHitResult _outhit)))) 1e+02)) 100)) (Math|Conversions|ToFloat(Integer) (* (Class|KismetMathLibrary|Round64 (/ (.Y (Math|Vector|BreakVector (.Location (Collision|BreakHitResult _outhit)))) 1e+02)) 100)) (.Z (Math|Vector|BreakVector (.Location (Collision|BreakHitResult _outhit)))))))))

(fn CanConstruct
  (for _array_element 0
    (if (Variables|/Game/WW4/Blueprint/Other/BP_BuildingGridCell.BP_BuildingGridCell_C|GetEnabled _array_element)
      (if (Variables|/Game/WW4/Blueprint/Other/BP_BuildingGridCell.BP_BuildingGridCell_C|GetBlock _array_element)
        (LocalVariables|SetBlocked true))))
  (return (not (LocalVariables|GetBlocked))))

(fn AddChildren
  (Utilities|Array|Clear (Variables|Default|GetCellArr))
  (for _index (range 0 24)
    (bind _returnvalue (Game|SpawnActorfromClass "/Game/WW4/Blueprint/Other/BP_BuildingGridCell.BP_BuildingGridCell_C" (Math|Transform|MakeTransform (+ (Math|Vector|MakeVector (Math|Conversions|ToFloat(Integer) (* (- (/ _index 5) 2) 100)) (Math|Conversions|ToFloat(Integer) (* (- (Math|Integer|%(Integer) _index 5) 2) 100)) 0.0) (Variables|Default|Getoffset))) "Undefined" "MultiplyWithRoot" 0 0))
    (Transformation|AttachActorToActor _returnvalue self "None" "KeepRelative" "KeepRelative" "KeepRelative" true)
    (Utilities|Array|Add (.CellArr (Variables|Default|GetCellArr)) 0)))
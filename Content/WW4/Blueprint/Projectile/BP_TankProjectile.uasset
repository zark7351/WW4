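; BP_TankProjectile is a tank shell projectile that explodes and deals damage when it hits something.
; On hit it spawns an explosion particle and sound at the impact point, then destroys itself.
; A RangeDamage flag switches between radial damage with falloff around the impact and direct damage to the hit actor only.
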(event EventBeginPlay)

(event Collision|EventActorBeginOverlap
  (params (OtherActor :type Actor%20Object%20Reference)))

(event EventTick
  (params (DeltaSeconds :type Float%20%28single-precision%29)))

(event EventOnHit
  (params (HitComponent :type Primitive%20Component%20Object%20Reference) (OtherActor :type Actor%20Object%20Reference) (OtherComp :type Primitive%20Component%20Object%20Reference) (NormalImpulse :type Vector :default "0, 0, 0") (Hit :type Hit%20Result%20Structure%20%28by%20ref%29))
  (bind _impactpoint (Collision|BreakHitResult Hit))
  (bind _damage (Variables|Default|GetDamage))
  (Effects|SpawnEmitteratLocation "/Game/StarterContent/Particles/P_Explosion.P_Explosion" _impactpoint (Math|Random|RandomRotator true))
  (Audio|PlaySoundatLocation "/Game/StarterContent/Audio/Explosion_Cue.Explosion_Cue" _impactpoint "0, 0, 0" 1.0 1.0 0.0 0 0 0 0)
  (if (Variables|Default|GetbRangeDamage)
    (Class|GameplayStatics|ApplyRadialDamagewithFalloff _damage (Variables|Default|GetMinimumDamage) _impactpoint (Variables|Default|GetDamageInnerRadius) (Variables|Default|GetDamageOuterRadius) (Variables|Default|GetDamageFalloff) "/Script/Engine.DamageType" 0 0 0 "ECC_Visibility")
    (else
      (Game|Damage|ApplyDamage OtherActor _damage 0 0)))
  (Actor|DestroyActor))

(fn ConstructionScript)
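; Base Blueprint for a tank projectile that explodes once it has travelled its maximum range.
; The construction script applies the speed variable to the projectile movement component and the radius variable to the collision sphere.
; BeginPlay records the start position, and Tick calls Explode when the horizontal distance from it reaches Range, ignoring height.
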(event EventBeginPlay
  (Variables|Default|SetStartPos (Transformation|GetActorLocation)))

(event Collision|EventActorBeginOverlap
  (params (OtherActor :type Actor%20Object%20Reference)))

(event EventTick
  (params (DeltaSeconds :type Float%20%28single-precision%29))
  (bind _returnvalue (Transformation|GetActorLocation))
  (bind _startpos (Variables|Default|GetStartPos))
  (bind _returnvalue_2 (- _returnvalue _startpos))
  (if (>= (Math|Vector|VectorLength (Math|Vector|MakeVector (.x _returnvalue_2) (.y _returnvalue_2) 0.0)) (Variables|Default|GetRange))
    (Class|ProjectileBase|Explode)))

(fn ConstructionScript
  (bind _projectilemovement (Variables|Default|GetProjectileMovement))
  (bind _speed (Variables|Default|GetSpeed))
  (Variables|/Script/Engine.ProjectileMovementComponent|SetInitialSpeed _projectilemovement _speed)
  (Variables|/Script/Engine.ProjectileMovementComponent|SetMaxSpeed _projectilemovement _speed)
  (Components|Sphere|SetSphereRadius (Variables|Default|GetCollisionSphere) (Variables|Default|GetRadius) true))
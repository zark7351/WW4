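; TestRocket is a projectile test Blueprint that builds an arced spline path between its Start and End components; it contains no movement logic.
; The InitSpline event passes both components' world locations to Init, which sets three world-space spline points.
; The midpoint is raised on Z by half the start-to-end distance, so arc height scales with range.
; The points use CurveClamped, Curve and Constant types respectively.
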(event Custom|InitSpline
  (CallFunction|Init (Transformation|GetWorldLocation (Variables|Default|GetStart)) (Transformation|GetWorldLocation (Variables|Default|GetEnd))))

(event EventBeginPlay)

(event Collision|EventActorBeginOverlap
  (params (OtherActor :type Actor%20Object%20Reference)))

(event EventTick
  (params (DeltaSeconds :type Float%20%28single-precision%29)))

(fn ConstructionScript)

(fn Init
  (params (start :type Vector) (end :type Vector))
  (bind _spline (Variables|Default|GetSpline))
  (Spline|SetSplinePoints _spline (Utilities|Array|MakeArray start (+ (/ (+ start end) 2.0) (Math|Vector|MakeVector 0.0 0.0 (/ (Math|Vector|VectorLength (- end start)) 2.0))) end) "World" true)
  (Spline|SetSplinePointType _spline 0 "CurveClamped" true)
  (Spline|SetSplinePointType _spline 1 "Curve" true)
  (Spline|SetSplinePointType _spline 2 "Constant" true))
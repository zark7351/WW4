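; BP_RocketPath is an actor that builds an arced spline path between a Start and an End position, named for rocket projectiles.
; On BeginPlay, InitSpline sets three world-space points, lifting the midpoint by a third of the start-to-end distance so the arc scales with range.
; All three point-type calls target index 0, so only the first point changes, ending as CurveClamped.
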(event EventBeginPlay
  (CallFunction|InitSpline (Variables|Default|GetStart) (Variables|Default|GetEnd)))

(event Collision|EventActorBeginOverlap
  (params (OtherActor :type Actor%20Object%20Reference)))

(event EventTick
  (params (DeltaSeconds :type Float%20%28single-precision%29)))

(fn ConstructionScript)

(fn InitSpline
  (params (Start :type Vector) (End :type Vector))
  (bind _spline (Variables|Default|GetSpline))
  (Spline|SetSplinePoints _spline (Utilities|Array|MakeArray Start (+ (/ (+ Start End) 2.0) (Math|Vector|MakeVector 0.0 0.0 (/ (Math|Vector|VectorLength (- End Start)) 3.0))) End) "World" true)
  (Spline|SetSplinePointType _spline 0 "CurveClamped" true)
  (Spline|SetSplinePointType _spline 0 "Curve" true)
  (Spline|SetSplinePointType _spline 0 "CurveClamped" true))
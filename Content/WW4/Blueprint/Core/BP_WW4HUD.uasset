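; BP_WW4HUD is the HUD class that creates the main UI widget and runs box-selection queries for units.
; BeginPlay adds WBP_Main to the viewport and keeps it as MainUI.
; While MainUI is selecting, DrawHUD scales its drag start and end points by viewport scale and queries for fully enclosed UnitBase actors.
; The query result is not used further in this graph.
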(event EventBeginPlay
  (bind _returnvalue (UserInterface|CreateWidget "/Game/WW4/Blueprint/UI/WBP_Main.WBP_Main_C"))
  (Variables|Default|SetMainUI _returnvalue)
  (UserInterface|Viewport|AddtoViewport _returnvalue 0))

(event Collision|EventActorBeginOverlap
  (params (OtherActor :type Actor%20Object%20Reference)))

(event EventTick
  (params (DeltaSeconds :type Float%20%28single-precision%29)))

(event EventDrawHUD
  (params (SizeX :type Integer) (SizeY :type Integer))
  (bind _returnvalue (Class|WidgetLayoutLibrary|GetViewportScale))
  (bind _mainui (Variables|Default|GetMainUI))
  (bind _mainui_2 (Variables|Default|GetMainUI))
  (Utilities|IsValid _mainui
    (:Is%20Valid
      (if (Variables|/Game/WW4/Blueprint/UI/WBP_Main.WBP_Main_C|GetSelecting _mainui)
        (Variables|Default|SetOutActors (Class|HUD|GetActorsinSelectionRectangle "/Script/WW4.UnitBase" (* _returnvalue (Variables|/Game/WW4/Blueprint/UI/WBP_Main.WBP_Main_C|GetStartPos _mainui_2)) (* _returnvalue (Variables|/Game/WW4/Blueprint/UI/WBP_Main.WBP_Main_C|GetEndPos _mainui_2)) false true))))))

(fn ConstructionScript)
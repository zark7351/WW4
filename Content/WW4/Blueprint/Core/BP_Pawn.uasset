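; Player pawn that pans across the map and confirms building placement, likely as a top-down strategy camera.
; IA_Move input and per-tick mouse screen-edge checks both feed movement input, with directions rotated 45 degrees to suit a diagonal view.
; R returns the pawn to the PlayerStart.
; Left mouse release calls Construct on the active BP_BuildingConstructor and, on success, destroys it and every BP_GridCell.
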(event Input|EnhancedActionEvents|EnhancedInputActionIA_Move
  (params (ActionValue :type Vector%202D%20Structure) (ElapsedSeconds :type Float%20%28double-precision%29) (TriggeredSeconds :type Float%20%28double-precision%29) (InputAction :type Input%20Action%20Object%20Reference :default "/Game/WW4/Blueprint/Input/IA_Move.IA_Move"))
  (bind _returnvalue (Class|KismetMathLibrary|GetRotated2D ActionValue 45.0))
  (bind (_x _y) (Math|Vector2D|BreakVector2D _returnvalue))
  (:Triggered
    (Pawn|Input|AddMovementInput (Math|Vector|MakeVector _x _y 0.0) 1e+01 false :!label _label))
  (:Ongoing
    (goto _label)))

(event EventTick
  (params (DeltaSeconds :type Float%20%28single-precision%29))
  (bind _returnvalue (Viewport|GetViewportSize))
  (bind _returnvalue_2 (Class|WidgetLayoutLibrary|GetViewportScale))
  (bind _returnvalue_3 (Math|Vector2D|MakeVector2D 0.0 1.0))
  (bind _returnvalue_4 (Math|Vector2D|MakeVector2D -1.0 0.0))
  (bind _returnvalue_5 (Math|Vector2D|MakeVector2D 1.0 0.0))
  (bind _returnvalue_6 (Math|Vector2D|MakeVector2D 0.0 -1.0))
  (bind _returnvalue_7 (Class|KismetMathLibrary|GetRotated2D _returnvalue_3 -45.0))
  (bind _returnvalue_8 (Class|KismetMathLibrary|GetRotated2D _returnvalue_4 -45.0))
  (bind _returnvalue_9 (Class|KismetMathLibrary|GetRotated2D _returnvalue_5 -45.0))
  (bind _returnvalue_10 (Class|KismetMathLibrary|GetRotated2D _returnvalue_6 -45.0))
  (bind _returnvalue_11 (/ _returnvalue _returnvalue_2))
  (bind (_x _y) (Math|Vector2D|BreakVector2D _returnvalue_11))
  (bind (_x_2 _y_2) (Math|Vector2D|BreakVector2D _returnvalue_7))
  (bind (_x_3 _y_3) (Math|Vector2D|BreakVector2D _returnvalue_8))
  (bind (_x_4 _y_4) (Math|Vector2D|BreakVector2D _returnvalue_9))
  (bind (_x_5 _y_5) (Math|Vector2D|BreakVector2D _returnvalue_10))
  (bind _returnvalue_12 (Class|WidgetLayoutLibrary|GetMousePositiononViewport))
  (Utilities|FlowControl|Sequence
    (:then_0
      (if (< (/ (.X (Math|Vector2D|BreakVector2D _returnvalue_12)) _x) 0.01)
        (Pawn|Input|AddMovementInput (Math|Vector|MakeVector _x_3 _y_3 0.0) 1e+01 false)
        (elif (> (/ (.X (Math|Vector2D|BreakVector2D _returnvalue_12)) _x) 0.99)
          (Pawn|Input|AddMovementInput (Math|Vector|MakeVector _x_4 _y_4 0.0) 1e+01 false))))
    (:then_1
      (if (< (/ (.Y (Math|Vector2D|BreakVector2D _returnvalue_12)) _y) 0.01)
        (Pawn|Input|AddMovementInput (Math|Vector|MakeVector _x_5 _y_5 0.0) 1e+01 false)
        (elif (> (/ (.Y (Math|Vector2D|BreakVector2D _returnvalue_12)) _y) 0.99)
          (Pawn|Input|AddMovementInput (Math|Vector|MakeVector _x_2 _y_2 0.0) 1e+01 false))))))

(event Collision|EventActorBeginOverlap
  (params (OtherActor :type Actor%20Object%20Reference)))

(event Input|MouseEvents|LeftMouseButton
  (params (Key :type Key%20Structure :default "None"))
  (:Released
    (CallFunction|Construct)))

(event Input|KeyboardEvents|R
  (params (Key :type Key%20Structure :default "None"))
  (:Pressed
    (bind _returnvalue (Actor|GetActorOfClass "/Script/Engine.PlayerStart"))
    (Transformation|SetActorLocation (Transformation|GetActorLocation _returnvalue) false false)))

(fn ConstructionScript)

(fn Construct
  (bind _returnvalue (Actor|GetActorOfClass "/Game/WW4/Blueprint/Other/BP_BuildingConstructor.BP_BuildingConstructor_C"))
  (Utilities|IsValid _returnvalue
    (:Is%20Valid
      (bind _returnvalue_2 (Class|BuildingConstructor|Construct _returnvalue))
      (if _returnvalue_2
        (Actor|DestroyActor _returnvalue)
        (bind _outactors (Actor|GetAllActorsOfClass "/Game/WW4/Blueprint/Other/BP_GridCell.BP_GridCell_C"))
        (for _array_element _outactors
          (Actor|DestroyActor _array_element))))))
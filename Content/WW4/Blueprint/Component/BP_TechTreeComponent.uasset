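; Player controller component that manages the tech tree of constructible buildings and vehicles, tracking which items are built and unlocked.
; On BeginPlay it loads all rows from the building and vehicle data tables, unlocking those in the initial unlock list.
; When a new item type is first constructed, it unlocks items whose prerequisites are all built and refreshes the HUD's construct list.
; It also provides item lookup by ID.
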(event EventBeginPlay
  (CallFunction|InitConstructItems))

(event EventTick
  (params (DeltaSeconds :type Float%20%28single-precision%29)))

(fn InitConstructItems
  (bind _vehicletable (Variables|Default|GetVehicleTable))
  (bind _buildingtable (Variables|Default|GetBuildingTable))
  (Utilities|FlowControl|Sequence
    (:then_0
      (Utilities|Array|Clear (Variables|Default|GetAllItems))
      (Utilities|Array|Clear (Variables|Default|GetUnlockedItems))
      (Utilities|FlowControl|Sequence
        (:then_0
          (bind _outrownames (DataTable|GetDataTableRowNames _buildingtable))
          (for _array_element _outrownames
            (bind _returnvalue (Utilities|GetDataTableRow _buildingtable _array_element)
              (:then
                (Utilities|Array|Add (Variables|Default|GetAllItems) _returnvalue)
                (if (Utilities|Array|ContainsItem (Variables|Default|GetInitUnlockItems) (.ItemID (Utilities|Struct|BreakItemProductionInfoBase _returnvalue)))
                  (Utilities|Array|Add (Variables|Default|GetUnlockedItems) _returnvalue))))))
        (:then_1
          (bind _outrownames_2 (DataTable|GetDataTableRowNames _vehicletable))
          (for _array_element_2 _outrownames_2
            (bind _returnvalue_2 (Utilities|GetDataTableRow _vehicletable _array_element_2)
              (:then
                (Utilities|Array|Add (Variables|Default|GetAllItems) _returnvalue_2)
                (if (Utilities|Array|ContainsItem (Variables|Default|GetInitUnlockItems) (.ItemID (Utilities|Struct|BreakItemProductionInfoBase _returnvalue_2)))
                  (Utilities|Array|Add (Variables|Default|GetUnlockedItems) _returnvalue_2))))))))))

(fn OnNewItemConstructed
  (params (ItemID :type Integer))
  (bind _builtitems (Variables|Default|GetBuiltItems))
  (bind _unlockeditems (Variables|Default|GetUnlockedItems))
  (if (not (Utilities|Set|Contains _builtitems ItemID))
    (Utilities|Set|Add _builtitems ItemID)
    (for _array_element (Variables|Default|GetAllItems)
      (if (not (== ItemID (.ItemID (Utilities|Struct|BreakItemProductionInfoBase _array_element))))
        (if (not (Utilities|Array|ContainsItem (Variables|Default|GetUnlockedItems) _array_element))
          (bind _result (CallFunction|CheckPrerequisite _array_element))
          (if _result
            (if (not (Utilities|Array|ContainsItem _unlockeditems _array_element))
              (Utilities|Array|Add _unlockeditems _array_element)
              (bind _asww4player_controller (Utilities|Casting|CastToWW4PlayerController (Components|GetOwner)))
              (Default|RefreshConstructItems (.AsBP%20WW4HUD (Utilities|Casting|CastToBP_WW4HUD (HUD|GetHUD _asww4player_controller))) (Variables|Default|GetUnlockedItems)))))))))

(fn CheckPrerequisite
  (params (CheckItem :type Item%20Production%20Info%20Base%20Structure))
  ;[1 1 1] 检查当前Item是否可以解锁
  (for _array_element (.PrerequisiteItemsID (Utilities|Struct|BreakItemProductionInfoBase CheckItem))
    (if (not (Utilities|Set|Contains (Variables|Default|GetBuiltItems) _array_element))
      (return false)))
  (return true))

(fn FindItemInfobyID
  (params (ID :type Integer))
  (for _array_element (Variables|Default|GetAllItems)
    (if (== ID (.ItemID (Utilities|Struct|BreakItemProductionInfoBase _array_element)))
      (return _array_element)))
  (return ""))